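; Game mode that runs the game's money economy and spawns ambient road traffic.
; A looping timer adds the per-cycle income to Money; AddIncome raises that income, and Pay deducts a cost only if affordable, returning success.
; A second looping timer spawns either a car or a pedestrian at a random road actor's location while the count of mobile actors stays under a cap.
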(event `CollectIncome`
  (set `self.Money` (+ (`self.Money`) (`self.IncomePerCycle`))))

(event `self.ReceiveBeginPlay`
  (`KismetSystemLibrary.K2_SetTimerDelegate` (delegate `CollectIncome`) 5.0 true)
  (`KismetSystemLibrary.K2_SetTimerDelegate` (delegate `SpawnTraffic`) 2.0 true))

(event `SpawnTraffic`
  (bind _outactors (`GameplayStatics.GetAllActorsOfClass` "/Game/GAME/BP/Mobile/BP_Mobile.BP_Mobile_C"))
  (if (< (`KismetArrayLibrary.Array_Length` _outactors) 30)
    (bind _outactors_2 (`GameplayStatics.GetAllActorsOfClass` "/Game/GAME/BP/Building/BP_Road.BP_Road_C"))
    (if (not (`KismetArrayLibrary.Array_IsEmpty` _outactors_2))
      (if (`KismetMathLibrary.RandomBool`)
        (bind _returnvalue (`KismetMathLibrary.MakeTransform` (`self.K2_GetActorLocation` (`KismetArrayLibrary.Array_Random` _outactors_2))))
        (`|SpawnActorFromClass` "/Game/GAME/BP/Mobile/BP_Car.BP_Car_C" _returnvalue "Undefined" "MultiplyWithRoot" null null)
        (else
          (`|SpawnActorFromClass` "/Game/GAME/BP/Mobile/BP_Pedestrian.BP_Pedestrian_C" _returnvalue "Undefined" "MultiplyWithRoot" null null))))))

(fn `AddIncome`
  (params (Amount :type Integer))
  (set `self.IncomePerCycle` (+ (`self.IncomePerCycle`) Amount)))

(fn `Pay`
  (params (Amount :type Integer))
  (returns (Ok :type Boolean))
  ;[0.031 0.6823 0.09084 0.5] HE GET THE AMOUNT OF THE ITEM, VERIFY IF PLAYER HAVE ENOUGH MONEY, IF YES HE TAKE THE AMOUNT FROM THE MONEY, AND DECLINE IF NO
  (if (>= (`self.Money`) Amount)
    (set `self.Money` (- (`self.Money`) (`local.Amount`)))
    (return true)
    (else
      (return false))))

(fn `UserConstructionScript`)