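; BP_CameraPawn is a player camera pawn that pans, rotates and zooms over a bounded map.
; Enhanced Input actions move it along its forward and right vectors, apply frame-rate-scaled yaw rotation, and set a clamped target zoom.
; Tick smoothly interpolates the spring arm length toward that target, then clamps the pawn's X and Y position to a square MapLimit around the world origin.
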(event `EnhancedInput|/Game/GAME/Input/Action/IA_Move`
  (params (ActionValue :type "Vector2D Structure") (ElapsedSeconds :type "Float (double-precision)") (TriggeredSeconds :type "Float (double-precision)") (InputAction :type "InputAction Object Reference" :default "/Game/GAME/Input/Action/IA_Move.IA_Move"))
  (bind (_x _y) (`KismetMathLibrary.BreakVector2D` ActionValue))
  ;[0 0.4428 1] CAMERA MOVEMENT
  (:`Triggered`
    (`self.AddMovementInput` (`self.GetActorForwardVector`) _y)
    (`self.AddMovementInput` (`self.GetActorRightVector`) _x)))

(event `EnhancedInput|/Game/GAME/Input/Action/IA_Rotate`
  (params (ActionValue :type "Float (double-precision)") (ElapsedSeconds :type "Float (double-precision)") (TriggeredSeconds :type "Float (double-precision)") (InputAction :type "InputAction Object Reference" :default "/Game/GAME/Input/Action/IA_Rotate.IA_Rotate"))
  ;[0 1 0.07601 0.5] CAMERA ROTATION
  (:`Triggered`
    (`self.K2_AddActorWorldRotation` (`KismetMathLibrary.MakeRotator` 0.0 0.0 (* (* ActionValue 90.0) (`GameplayStatics.GetWorldDeltaSeconds`))))))

(event `EnhancedInput|/Game/GAME/Input/Action/IA_Zoom`
  (params (ActionValue :type "Float (double-precision)") (ElapsedSeconds :type "Float (double-precision)") (TriggeredSeconds :type "Float (double-precision)") (InputAction :type "InputAction Object Reference" :default "/Game/GAME/Input/Action/IA_Zoom.IA_Zoom"))
  ;[1 0.3564 0 0.5] TARGET ZOOM
  (:`Triggered`
    (set `self.TargetZoom` (`KismetMathLibrary.FClamp` (- (`self.TargetZoom`) (* ActionValue 200.0)) 500.0 4000.0))))

(event `self.ReceiveTick`
  (params (DeltaSeconds :type "Float (single-precision)"))
  (bind _maplimit (`self.MapLimit`))
  (bind _returnvalue (* _maplimit -1.0))
  ;[0.02102 0.15 0.02538 0.5] TICK
  ;;[1 0.0691 0 0.5] CAMERA ZOOM
  (set `SpringArmComponent.TargetArmLength` (`KismetMathLibrary.FInterpTo` (`SpringArmComponent.TargetArmLength` (`self.SpringArm`)) (`self.TargetZoom`) (`GameplayStatics.GetWorldDeltaSeconds`) 8.0) (`self.SpringArm`))
  (`self.K2_SetActorLocation` (`KismetMathLibrary.MakeVector` (`KismetMathLibrary.FClamp` (.x (`self.K2_GetActorLocation`)) _returnvalue _maplimit) (`KismetMathLibrary.FClamp` (.y (`self.K2_GetActorLocation`)) _returnvalue _maplimit) (.z (`self.K2_GetActorLocation`)))))

(fn `UserConstructionScript`)