(event `self.ReceiveBeginPlay`
  ; ADD THE MAPPING CONTEXT
  (`EnhancedInputSubsystemInterface.AddMappingContext` (subsystem `EnhancedInputLocalPlayerSubsystem`) "/Game/GAME/Input/IMC_Default.IMC_Default" 0 (struct))
  (bind _returnvalue (`GameplayStatics.GetActorOfClass` "/Game/GAME/BP/Grid/BP_GridManager.BP_GridManager_C"))
  (set `self.GridManager` _returnvalue)
  ;[0.003341 0.15 0.1336 0.5] GET THE GAME MODE
  (bind _asbp_game_mode (cast `/Game/GAME/BP/Core/BP_GameMode` (`GameplayStatics.GetGameMode`)))
  (set `self.MyGameMode` _asbp_game_mode)
  ; CREATE THE HUD AND ADD IT TO THE VIEWPORT TO MAKE IT VISIBLE
  (bind _returnvalue_2 (`|CreateWidget` "/Game/GAME/UI/WPB_HUD.WPB_HUD_C"))
  (`UserWidget.AddToViewport` _returnvalue_2 0))

(event `self.ReceiveTick`
  (params (DeltaSeconds :type "Float (single-precision)"))
  (bind (_hitresult _returnvalue) (`self.GetHitResultUnderCursorByChannel` "TraceTypeQuery1"))
  ;[0.01345 1 0.05453 0.5] GET THE SELECTIONNED CELL, THEN TP THE GREEN HIGHLIGHT ON IT
  (if _returnvalue
    (bind _cell (`/Game/GAME/BP/Grid/BP_GridManager.WorldToGrid` (`self.GridManager`) (`.ImpactPoint` (`GameplayStatics.BreakHitResult` _hitresult))))
    (bind _output_get (set `self.HoveredCell` _cell))
    (`/Game/GAME/BP/Grid/BP_GridManager.ShowCell` (`self.GridManager`) _output_get)))

(event `EnhancedInput|/Game/GAME/Input/Action/IA_Build`
  (params (ActionValue :type Boolean) (ElapsedSeconds :type "Float (double-precision)") (TriggeredSeconds :type "Float (double-precision)") (InputAction :type "InputAction Object Reference" :default "/Game/GAME/Input/Action/IA_Build.IA_Build"))
  ;[1 0 0.8823 0.5] VERIFY IF CAN BUILD, THEN GET THE CENTER POINT POSITION OF THE CELL, THEN VERIFY IF THE PLAYER CAN PAY AND IF YES BUILD THE BULDING AND FINALLY ADD THE CELL TO THE OCCUPY LIST
  (:`Started`
    (bind _ok (`/Game/GAME/BP/Grid/BP_GridManager.CanBuild` (`self.GridManager`) (`self.HoveredCell`)))
    (if _ok
      (bind _returnvalue (`|GetDataTableRow` "/Game/GAME/BP/DATA/DT_Buildings.DT_Buildings" (`self.SelectedBulding`))
        (:`then`
          (bind (_name _mesh _cost _income _class) (break `/Game/GAME/BP/DATA/S_Building` _returnvalue))
          (bind _ok_2 (`/Game/GAME/BP/Core/BP_GameMode.Pay` (`self.MyGameMode`) _cost))
          (set `self.Class` _class)
          (if _ok_2
            (bind _position (`/Game/GAME/BP/Grid/BP_GridManager.GridToWorld` (`self.GridManager`) (`self.HoveredCell`)))
            (bind _returnvalue_2 (`|SpawnActorFromClass` (`self.Class`) (`KismetMathLibrary.MakeTransform` _position) "Undefined" "MultiplyWithRoot" null (`self.HoveredCell`) (`self.SelectedBulding`) null))
            (`/Game/GAME/BP/Grid/BP_GridManager.OccupyCell` (`self.GridManager`) (`self.HoveredCell`) _returnvalue_2)))))))

(event `EnhancedInput|/Game/GAME/Input/Action/IA_Destroy`
  (params (ActionValue :type Boolean) (ElapsedSeconds :type "Float (double-precision)") (TriggeredSeconds :type "Float (double-precision)") (InputAction :type "InputAction Object Reference" :default "/Game/GAME/Input/Action/IA_Destroy.IA_Destroy"))
  ;[1 0 0.06491 0.5] DELETE BULDING
  (:`Started`
    (`/Game/GAME/BP/Grid/BP_GridManager.FreeCell` (`self.GridManager`) (`self.HoveredCell`))))

(fn `UserConstructionScript`)