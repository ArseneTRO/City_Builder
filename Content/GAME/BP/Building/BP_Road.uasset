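; BP_Road is a grid-placed road building piece that adapts its shape to neighbouring road cells.
; UpdateShape takes the grid and asks it whether each of the four orthogonally adjacent cells is a road.
; It shows or hides the matching arm component on each axis, forming straights, corners and junctions from one Blueprint.
; The event graph is unused, so the shape changes only when UpdateShape is called.
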(fn `UpdateShape`
  (params (Grid :type "/Game/GAME/BP/Grid/BP_GridManager Object Reference"))
  ;[0.006911 0.06192 0.15 0.5] ADAPT THE SHAPE IN FUNCTION OF HIS NEIGHBOORS. IF (CELL + (1;0)) = ROADS, THEN ARM X PLUS = TRUE = VISIBLE
  (bind _output_get (set `self.Grid` Grid))
  (bind _road (`/Game/GAME/BP/Grid/BP_GridManager.IsRoad` _output_get (+ (`self.Cell`) (make `IntPoint` 1))))
  (`SceneComponent.SetVisibility` (`self.ArmXPlus`) _road false)
  (bind _road_2 (`/Game/GAME/BP/Grid/BP_GridManager.IsRoad` (`self.Grid`) (+ (`self.Cell`) (make `IntPoint` -1))))
  (`SceneComponent.SetVisibility` (`self.ArmXMinus`) _road_2 false)
  (bind _road_3 (`/Game/GAME/BP/Grid/BP_GridManager.IsRoad` (`self.Grid`) (+ (`self.Cell`) (make `IntPoint` 0 1))))
  (`SceneComponent.SetVisibility` (`self.ArmYPlus`) _road_3 false)
  (bind _road_4 (`/Game/GAME/BP/Grid/BP_GridManager.IsRoad` (`self.Grid`) (+ (`self.Cell`) (make `IntPoint` 0 -1))))
  (`SceneComponent.SetVisibility` (`self.ArmYMinus`) _road_4 false))

(fn `UserConstructionScript`
  (`parent.UserConstructionScript`))