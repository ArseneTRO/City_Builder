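; BP_Building is a data-driven building actor that contributes income to the game economy.
; On BeginPlay it looks up its row in DT_Buildings by RowName, stores it as Info, sets the Body mesh from it and adds the row's income through BP_GameMode's AddIncome.
; When destroyed, it passes the negated income to the same function to withdraw its contribution.
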(event `self.ReceiveBeginPlay`
  (bind (_info_name _info_mesh _info_cost _info_income) (break `/Game/GAME/BP/DATA/S_Building` (`self.Info`)))
  ;[0 0.7131 1 0.5] AT BEGIN PLAY, IT GET THE DATA TABLE, GET THE LINE THAT CONCERN HIM, READ IT AND TAKE THE MESH ASSOCIATED
  (bind _returnvalue (`|GetDataTableRow` "/Game/GAME/BP/DATA/DT_Buildings.DT_Buildings" (`self.RowName`))
    (:`then`
      (set `self.Info` _returnvalue)
      (`StaticMeshComponent.SetStaticMesh` (`self.Body`) _info_mesh)
      ;[0 0.118 0.15 0.5] ADD TO INCOME
      (bind _asbp_game_mode (cast `/Game/GAME/BP/Core/BP_GameMode` (`GameplayStatics.GetGameMode`)))
      (`/Game/GAME/BP/Core/BP_GameMode.AddIncome` _asbp_game_mode _info_income))))

(event `self.ReceiveDestroyed`
  ;[0.15 0 0.003412 0.5] DISABLE HIS PART OF THE INCOMES WHEN DESTROYED
  (bind _asbp_game_mode (cast `/Game/GAME/BP/Core/BP_GameMode` (`GameplayStatics.GetGameMode`)))
  (`/Game/GAME/BP/Core/BP_GameMode.AddIncome` _asbp_game_mode (* (`.Income_8_8BA1742F4FE43D513E7E95B8535227A5` (break `/Game/GAME/BP/DATA/S_Building` (`self.Info`))) -1)))

(fn `UserConstructionScript`)