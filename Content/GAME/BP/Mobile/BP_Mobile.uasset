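; BP_Mobile is an actor that wanders the grid's roads, keeping to the right of its travel direction.
; ChooseNextCell picks a random neighboring road cell, turning back only at dead ends, or destroys the actor if its current cell is not road.
; The target is offset sideways using the perpendicular of the travel direction.
; Tick moves at constant speed, snaps on arrival and chooses the next cell.
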(event `self.ReceiveBeginPlay`
  ;[0.6071 0.632 1 0.5] WHEN BEGIN PLAY, GET THE GRID, SET THE CURRENT CELL AND PREVIOUS CELL TO THE ACTUAL CELL, THEN LAUNCH CHOOSE NEXT CELL
  (bind _returnvalue (`GameplayStatics.GetActorOfClass` "/Game/GAME/BP/Grid/BP_GridManager.BP_GridManager_C"))
  (set `self.Grid` _returnvalue)
  (bind _cell (`/Game/GAME/BP/Grid/BP_GridManager.WorldToGrid` (`self.Grid`) (`self.K2_GetActorLocation`)))
  (bind _output_get (set `self.CurrentCell` _cell))
  (set `self.PreviousCell` _output_get)
  (`self.ChooseNextCell`))

(event `self.ReceiveTick`
  (params (DeltaSeconds :type "Float (single-precision)"))
  (bind _returnvalue (* DeltaSeconds (`self.Speed`)))
  ;[0 0.2794 1 0.5] EVERY SECONDS, WE CHECK IF THE DESTINATION CAN BE REACHED IN THE NEXT STEP OR NOT. IF YES, THEN WE SET THAT WE ARRIVE AT THE DESTINATION, AND WE LAUNCH "CHOOSE NEXT CELL" TO CHOOSE THE NEXT DESTINATION. IF NO, WE JUST DO ANOTHER STEP
  (if (<= (`KismetMathLibrary.Distance2D` (`KismetMathLibrary.Conv_VectorToVector2D` (`self.K2_GetActorLocation`)) (`KismetMathLibrary.Conv_VectorToVector2D` (`self.Destination`))) _returnvalue)
    (`self.K2_SetActorLocation` (`self.Destination`))
    (set `self.PreviousCell` (`self.CurrentCell`))
    (set `self.CurrentCell` (`self.NextCell`))
    (`self.ChooseNextCell`)
    (else
      (`self.K2_AddActorWorldOffset` (* _returnvalue (`KismetMathLibrary.Normal` (- (`self.Destination`) (`self.K2_GetActorLocation`))))))))

(fn `ChooseNextCell`
  ;[0.4704 0 1 0.5] CHECK IF THE ACTOR IS ON A ROAD, SO HE DOESN'T DESTROY HIM AND HE CLEAR THE CANDIDATES LIST TO REMOVE THE PREVIOUS CANDIDATES FROM THE PREVIOUS CELLE. IF NOT ON A ROAD, DESTROY ACTOR
  (bind _road (`/Game/GAME/BP/Grid/BP_GridManager.IsRoad` (`self.Grid`) (`self.CurrentCell`)))
  (if _road
    (`KismetArrayLibrary.Array_Clear` (`self.Candidates`))
    ;[0.9947 0.03842 1 0.5] LOOP (CHECK EVERY POSSIBILITY EXCEPT THE PREVIOUS CELL
    (for _array_element (`self.Directions`)
      (bind _returnvalue (+ (`self.CurrentCell`) _array_element))
      (bind _road_2 (`/Game/GAME/BP/Grid/BP_GridManager.IsRoad` (`self.Grid`) _returnvalue))
      (if (and _road_2 (not (`KismetMathLibrary.Equal_IntPointIntPoint` (`self.PreviousCell`) _returnvalue)))
        (`KismetArrayLibrary.Array_Add` (`self.Candidates`) _returnvalue)))
    ;[1 0 0.5391 0.5] END OF THE LOOP (CHECK IF THERE IS CANDIDATES THAT ARE NOT THE PREVIOUS CELL, OTHERWISE, ADD THE PREVIOUS CELL AS THE ONLY CANDIDATE)
    (`|ExecutionSequence`
      (:`then_0`
        (if (`KismetArrayLibrary.Array_IsEmpty` (`self.Candidates`))
          (`KismetArrayLibrary.Array_Add` (`self.Candidates`) (`self.PreviousCell`))))
      (:`then_1`
        ;[1 0 0.03836 0.5] GET A RANDOM DIRECTION IF THERE IS ALREADY DIRECTION SUGGERED IN CANDIDATES
        (set `self.NextCell` (`KismetArrayLibrary.Array_Random` (`self.Candidates`)))
        (bind _position (`/Game/GAME/BP/Grid/BP_GridManager.GridToWorld` (`self.Grid`) (`self.CurrentCell`)))
        (bind _position_2 (`/Game/GAME/BP/Grid/BP_GridManager.GridToWorld` (`self.Grid`) (`self.NextCell`)))
        ;[1 0.5615 0 0.5] GET THE RIGHT SIDE OF THE VERTEX (SO REVERSE THE VERTEX AND NEGATE HIS FIRST DATA)
        (set `self.Destination` (+ (* (`KismetMathLibrary.MakeVector` (* (.y (`KismetMathLibrary.Normal` (- _position_2 _position))) -1.0) (.x (`KismetMathLibrary.Normal` (- _position_2 _position)))) (`self.Offset`)) _position_2))
        ;[0.538 1 0 0.5] SET THE FINAL DECISION
        (`self.K2_SetActorRotation` (`KismetMathLibrary.FindLookAtRotation` (`self.K2_GetActorLocation`) (`self.Destination`)))))
    (else
      (`self.K2_DestroyActor`))))

(fn `UserConstructionScript`)