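; Grid manager actor for tile-based building, tracking which cells are occupied and by which building.
; BeginPlay lays out cells as mesh instances, with helpers converting between world and grid coordinates relative to the actor.
; A highlight mesh moves to the shown cell, turning green or red by buildability.
; An Occupancy map backs placement checks and demolition; occupying or freeing a cell prompts it and neighboring BP_Road actors to update their shape.
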(event `self.ReceiveBeginPlay`
  ;[0 0.3882 1 0.5] CREER LES CASES AU LANCEMENT
  (for _index (range (`self.CellCountX`))
    (for _index_2 (range (`self.CellCountY`))
      (bind _position (`self.GridToWorld` (make `IntPoint` _index _index_2)))
      (`InstancedStaticMeshComponent.AddInstance` (`self.Cells`) (`KismetMathLibrary.MakeTransform` (+ _position (0.0 0.0 1.0)) (struct) (0.95 0.95 1.0)) true))))

(fn `CanBuild`
  (params (Cell :type "IntPoint Structure"))
  (returns (Ok :type Boolean))
  ; VERIFY IF THE CELL IS FREE TO BUILD OR NOT
  (bind _inside (`self.IsInsideGrid` Cell))
  (return (and _inside (not (`BlueprintMapLibrary.Map_Contains` (`self.Occupancy`) Cell)))))

(fn `FreeCell`
  (params (Cell :type "IntPoint Structure"))
  (bind _value (`BlueprintMapLibrary.Map_Find` (`self.Occupancy`) Cell))
  ; FREE AN OCCUPY CELL (DESTROY BUILDINGS)
  (`/Engine/EditorBlueprintResources/StandardMacros.IsValid` _value
    (:`Is Valid`
      (`self.K2_DestroyActor` _value)
      (`BlueprintMapLibrary.Map_Remove` (`self.Occupancy`) Cell)
      (`self.RefreshNeighbors` Cell))))

(fn `GridToWorld`
  (params (Cell :type "IntPoint Structure"))
  (returns (Position :type "Vector Structure"))
  (bind (_x _y) (break `IntPoint` Cell))
  (bind _cellsize (`self.CellSize`))
  (bind _returnvalue (/ _cellsize 2.0))
  (return (`KismetMathLibrary.MakeVector` (+ (* _x _cellsize) (.x (`self.K2_GetActorLocation`)) _returnvalue) (+ (* _y _cellsize) (.y (`self.K2_GetActorLocation`)) _returnvalue) (.z (`self.K2_GetActorLocation`)))))

(fn `IsInsideGrid`
  (params (Cell :type "IntPoint Structure"))
  (returns (Inside :type Boolean))
  (bind (_x _y) (break `IntPoint` Cell))
  (return (and (>= _x 0) (< _x (`self.CellCountX`)) (>= _y 0) (< _y (`self.CellCountY`)))))

(fn `IsRoad`
  (params (Cell :type "IntPoint Structure"))
  (returns (Road :type Boolean))
  (return (`.bSuccess` (cast `/Game/GAME/BP/Building/BP_Road` (`BlueprintMapLibrary.Map_Find` (`self.Occupancy`) Cell) :!pure true))))

(fn `OccupyCell`
  (params (Cell :type "IntPoint Structure") (Building :type "Actor Object Reference"))
  ; ADD THE CELL TO THE LIST
  (`BlueprintMapLibrary.Map_Add` (`self.Occupancy`) Cell Building)
  (`self.RefreshNeighbors` Cell))

(fn `RefreshCell`
  (params (Cell :type "IntPoint Structure"))
  (bind _asbp_road (cast `/Game/GAME/BP/Building/BP_Road` (`BlueprintMapLibrary.Map_Find` (`self.Occupancy`) Cell)))
  (`/Game/GAME/BP/Building/BP_Road.UpdateShape` _asbp_road self))

(fn `RefreshNeighbors`
  (params (Cell :type "IntPoint Structure"))
  ; IT USE THE REFRESH CELL FUNCTION ON HIMSELF THEN ON ALL HIS NEIGHBORS
  (`self.RefreshCell` Cell)
  (for _array_element (`self.Directions[0]`)
    (`self.RefreshCell` (+ Cell _array_element))))

(fn `ShowCell`
  (params (Cell :type "IntPoint Structure"))
  ;[0 1 0.08104 0.5] TP LA CELL HIGHLIGHT AU DESSUS DE LA CELLE SELECTIONNEE
  (bind _position (`self.GridToWorld` Cell))
  (`SceneComponent.K2_SetWorldLocation` (`self.Highlight`) (+ _position (0.0 0.0 2.0)) false false)
  (bind _ok (`self.CanBuild` Cell))
  (if _ok
    (`PrimitiveComponent.SetMaterial` (`self.Highlight`) 0 (`self.GreenMaterial`))
    (else
      (`PrimitiveComponent.SetMaterial` (`self.Highlight`) 0 (`self.RedMaterial`)))))

(fn `UserConstructionScript`)

(fn `WorldToGrid`
  (params (Position :type "Vector Structure"))
  (returns (Cell :type "IntPoint Structure"))
  (bind _cellsize (`self.CellSize`))
  ;[0.15 1 0.15 0.5] CONVERT WORLD POSITION INTO GRID COORDONATES
  (return (make `IntPoint` (`KismetMathLibrary.FFloor` (/ (- (.x Position) (.x (`self.K2_GetActorLocation`))) _cellsize)) (`KismetMathLibrary.FFloor` (/ (- (.y Position) (.y (`self.K2_GetActorLocation`))) _cellsize)))))